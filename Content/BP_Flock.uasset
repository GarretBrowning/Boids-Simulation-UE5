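; Flock manager that drives boid flocking for every BP_Boid found in the level at BeginPlay.
; Each Tick it first adds steering to every boid's acceleration, then calls ApplyMovement on each in a second pass.
; Alignment and cohesion use clamped steering averaged over all other boids, with no radius check, and cohesion draws debug arrows.
; Separation is summed but its calculation is disconnected, and earlier vector functions and spawning logic remain unwired.
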(event `self.ReceiveBeginPlay`
  ;[0.2191 1 0.4284] Get All Boids and Add to Array
  (bind _outactors (`GameplayStatics.GetAllActorsOfClass` "/Game/BP_Boid.BP_Boid_C"))
  (set `self.Boids` _outactors))

(event `self.ReceiveTick`
  (params (DeltaSeconds :type "Float (single-precision)"))
  (`|ExecutionSequence`
    (:`then_0`
      (for _array_element (`self.Boids`)
        (`self.CalculateTotalAcceleration` _array_element)))
    (:`then_1`
      (for _array_element_2 (`self.Boids`)
        (`/Game/BP_Boid.ApplyMovement` _array_element_2 (0.0 0.0 0.0))))))

(event `Debug`
  ;[0.2191 1 0.4284] Debugging
  (`|ExecutionSequence`
    (:`then_0`
      (`KismetSystemLibrary.PrintString` (`KismetStringLibrary.Concat_StrStr` "Number of Boids: " (`KismetStringLibrary.Conv_IntToString` (`KismetArrayLibrary.Array_Length` (`self.Boids`)))) true true (struct :`G` 0.66 :`B` 1.0 :`A` 1.0) (`GameplayStatics.GetWorldDeltaSeconds`)))))

(fn `Alignment_R`
  (params (CurrentBoid :type "/Game/BP_Boid Object Reference"))
  (returns (Alignment :type "Vector Structure"))
  (locals (AlignmentSteer :type "Vector Structure") (NeighbouringBoidsVelocities :type "Array of Vector Structure") (MaxAlignmentForce :type "Float (double-precision)" :default 0.4))
  (bind _currentboid (`local.CurrentBoid`))
  (for _array_element (`self.Boids`)
    (if (!= _array_element (`local.CurrentBoid`))
      (`KismetArrayLibrary.Array_Add` (`local.NeighbouringBoidsVelocities`) (`/Game/BP_Boid.Velocity` _array_element))))
  (if (> (`KismetArrayLibrary.Array_Length` (`local.NeighbouringBoidsVelocities`)) 0)
    (set `local.AlignmentSteer` (`KismetMathLibrary.ClampVectorSize` (* (`KismetMathLibrary.Normal` (- (`KismetMathLibrary.GetVectorArrayAverage` (`local.NeighbouringBoidsVelocities`)) (`/Game/BP_Boid.Velocity` _currentboid))) (`/Game/BP_Boid.MaxSpeed` _currentboid)) 0.0 (`local.MaxAlignmentForce`))))
  (return (`local.AlignmentSteer`)))

(fn `CalculateAlignmentVector`
  (params (Boid :type "/Game/BP_Boid Object Reference"))
  (returns (AlignmentV :type "Vector Structure"))
  (locals (DetectedBoidVelocities :type "Array of Vector Structure") (DetectionRadius :type "Float (double-precision)" :default 200.0) (AlignmentSteering :type "Vector Structure"))
  (bind _detectedboidvelocities (`local.DetectedBoidVelocities`))
  (for _array_element (`self.Boids`)
    (`KismetSystemLibrary.PrintString` (`KismetStringLibrary.Conv_BoolToString` (and (< (`KismetMathLibrary.Vector_Distance` (`self.K2_GetActorLocation` (`local.Boid`)) (`self.K2_GetActorLocation` _array_element)) (`/Game/BP_Boid.DetectionRadius` (`local.Boid`))) (!= _array_element (`local.Boid`)))))
    (if true
      (`KismetArrayLibrary.Array_Add` (`local.DetectedBoidVelocities`) (`/Game/BP_Boid.Velocity` _array_element))))
  (if (> (`KismetArrayLibrary.Array_Length` _detectedboidvelocities) 0)
    (set `local.AlignmentSteering` (* (`KismetMathLibrary.Normal` (- (`KismetMathLibrary.GetVectorArrayAverage` _detectedboidvelocities) (`/Game/BP_Boid.Velocity` (`local.Boid`)))) (`/Game/BP_Boid.MaxSpeed` (`local.Boid`)))))
  (return (`local.AlignmentSteering`)))

(fn `CalculateCohesionVector`
  (params (Boid :type "/Game/BP_Boid Object Reference"))
  (returns (CohesionV :type "Vector Structure"))
  (locals (CurrentBoidLocations :type "Array of Vector Structure"))
  (bind _returnvalue (`self.K2_GetActorLocation` Boid))
  (bind _averageboidlocation (`self.AverageBoidLocation`))
  ;[0.2191 1 0.4284] Calculating Average Boid Location
  (for _array_element (`self.Boids`)
    (`KismetArrayLibrary.Array_Add` (`local.CurrentBoidLocations`) (`self.K2_GetActorLocation` _array_element)))
  (set `self.AverageBoidLocation` (`KismetMathLibrary.GetVectorArrayAverage` (`local.CurrentBoidLocations`)))
  (`KismetSystemLibrary.DrawDebugArrow` _returnvalue _averageboidlocation)
  (return (* (`KismetMathLibrary.Normal` (- _averageboidlocation _returnvalue)) (`self.CohesionMultiplier`))))

(fn `CalculateFinalMovementVector`
  (params (CombinedMovement :type "Array of Vector Structure"))
  (returns (DeltaMovement :type "Vector Structure"))
  (return (`KismetMathLibrary.GetVectorArrayAverage` CombinedMovement)))

(fn `CalculateSeparationVector`
  (params (Boid :type "/Game/BP_Boid Object Reference"))
  (returns (SeparationV :type "Vector Structure"))
  (locals (BoidDirectionFromOtherBoids :type "Array of Vector Structure") (BoidDistanceFromOtherBoids :type "Array of Float (double-precision)") (TotalDistance :type "Float (double-precision)"))
  (bind _returnvalue (`self.K2_GetActorLocation` Boid))
  (bind _returnvalue_2 (`KismetMathLibrary.Normal` (`KismetMathLibrary.GetVectorArrayAverage` (`local.BoidDirectionFromOtherBoids`))))
  (for _array_element (`self.Boids`)
    (`KismetArrayLibrary.Array_Add` (`local.BoidDirectionFromOtherBoids`) (- _returnvalue (`self.K2_GetActorLocation` _array_element))))
  (`KismetSystemLibrary.DrawDebugArrow` _returnvalue (+ _returnvalue (* _returnvalue_2 200.0)) 0.0 (struct :`G` 0.692751 :`B` 1.0 :`A` 1.0))
  (return (* _returnvalue_2 (`self.SeparationMultiplier`))))

(fn `CalculateTotalAcceleration`
  (params (CurrentBoid :type "/Game/BP_Boid Object Reference"))
  (locals (Alignment :type "Vector Structure") (Cohesion :type "Vector Structure") (Separation :type "Vector Structure"))
  (bind _currentboid (`local.CurrentBoid`))
  (`|ExecutionSequence`
    (:`then_0`
      (bind _alignment (`self.Alignment_R` (`local.CurrentBoid`)))
      (set `local.Alignment` _alignment))
    (:`then_1`
      (bind _cohesion (`self.Cohesion_R` (`local.CurrentBoid`)))
      (set `local.Cohesion` _cohesion))
    (:`then_3`
      (set `/Game/BP_Boid.Acceleration` (+ (`/Game/BP_Boid.Acceleration` _currentboid) (`local.Cohesion`) (`local.Alignment`) (`local.Separation`)) _currentboid))))

(fn `Cohesion_R`
  (params (CurrentBoid :type "/Game/BP_Boid Object Reference"))
  (returns (Cohesion :type "Vector Structure"))
  (locals (CohesionSteer :type "Vector Structure") (NeighbouringBoidsPositions :type "Array of Vector Structure") (MaxCohesionForce :type "Float (double-precision)" :default 0.2))
  (bind _currentboid (`local.CurrentBoid`))
  (for _array_element (`self.Boids`)
    (if (!= _array_element (`local.CurrentBoid`))
      (`KismetArrayLibrary.Array_Add` (`local.NeighbouringBoidsPositions`) (`self.K2_GetActorLocation` _array_element))))
  (if (> (`KismetArrayLibrary.Array_Length` (`local.NeighbouringBoidsPositions`)) 0)
    (set `local.CohesionSteer` (`KismetMathLibrary.ClampVectorSize` (- (* (`KismetMathLibrary.Normal` (- (`KismetMathLibrary.GetVectorArrayAverage` (`local.NeighbouringBoidsPositions`)) (`self.K2_GetActorLocation` _currentboid))) (`/Game/BP_Boid.MaxSpeed` _currentboid)) (`/Game/BP_Boid.Velocity` (`local.CurrentBoid`))) 0.0 (`local.MaxCohesionForce`))))
  (`KismetSystemLibrary.DrawDebugArrow` (`self.K2_GetActorLocation` (`local.CurrentBoid`)) (`KismetMathLibrary.GetVectorArrayAverage` (`local.NeighbouringBoidsPositions`)))
  (return (`local.CohesionSteer`)))

(fn `Separatrion_R`
  (params (CurrentBoid :type "/Game/BP_Boid Object Reference"))
  (returns (Separation :type "Vector Structure"))
  (locals (SeparationSteer :type "Vector Structure") (NeighbouringBoidsDistancesAway :type "Array of Vector Structure") (MaxSeparationForce :type "Float (double-precision)" :default 0.6))
  (bind _currentboid (`local.CurrentBoid`))
  (for _array_element (`self.Boids`)
    (if (!= _array_element (`local.CurrentBoid`))
      (`KismetArrayLibrary.Array_Add` (`local.NeighbouringBoidsDistancesAway`) (/ (- (`self.K2_GetActorLocation` _array_element) (`self.K2_GetActorLocation` (`local.CurrentBoid`))) (`self.GetDistanceTo` (`local.CurrentBoid`) _array_element)))))
  (if (> (`KismetArrayLibrary.Array_Length` (`local.NeighbouringBoidsDistancesAway`)) 0)
    (set `local.SeparationSteer` (`KismetMathLibrary.ClampVectorSize` (* (`KismetMathLibrary.Normal` (- (`KismetMathLibrary.GetVectorArrayAverage` (`local.NeighbouringBoidsDistancesAway`)) (`/Game/BP_Boid.Velocity` _currentboid))) (`/Game/BP_Boid.MaxSpeed` _currentboid)) 0.0 (`local.MaxSeparationForce`))))
  (return (`local.SeparationSteer`)))

(fn `UserConstructionScript`)