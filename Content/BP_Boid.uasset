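; BP_Boid is a single boid actor that moves and turns according to a movement vector passed into its ApplyMovement event.
; ApplyMovement offsets the actor by that vector scaled by delta time and MovementSpeed, then smoothly interpolates its rotation toward the movement direction, using the current up vector.
; Tick only draws a debug arrow along the forward vector; an older forward-movement snippet is left unconnected.
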(event `ApplyMovement`
  (params (DeltaMovement :type "Vector Structure"))
  ;[1 1 1] Movement
  (`self.K2_AddActorWorldOffset` (* (* DeltaMovement (`GameplayStatics.GetWorldDeltaSeconds`)) (`self.MovementSpeed`)))
  (`self.K2_SetActorRotation` (`KismetMathLibrary.RInterpTo` (`self.K2_GetActorRotation`) (`KismetMathLibrary.MakeRotFromXZ` DeltaMovement (`self.GetActorUpVector`)) (`GameplayStatics.GetWorldDeltaSeconds`) 0.5)))

(event `self.ReceiveTick`
  (params (DeltaSeconds :type "Float (single-precision)"))
  (bind _returnvalue (`self.K2_GetActorLocation`))
  (`|ExecutionSequence`
    (:`then_0`
      (`KismetSystemLibrary.DrawDebugArrow` _returnvalue (+ _returnvalue (* (`self.GetActorForwardVector`) 100.0)) 3.0 (struct :`R` 0.019072 :`G` 1.0 :`A` 1.0) 0.0 1.0))
    (:`then_1`)))

(fn `UserConstructionScript`)